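; BP_FloorButton is a floor button actor that shows an on-screen message while the first-person player character stands in its trigger.
; On BeginPlay it creates a WBP_FloorButtonUI widget for player 0, stores it and adds it to the viewport.
; The Box component's begin and end overlap events, filtered by a cast to BP_FirstPersonCharacter, show and hide the widget's TextButtonMessage.
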(event OnComponentBeginOverlap(Box)
  (params (OverlappedComponent :type Primitive%20Component%20Object%20Reference) (OtherActor :type Actor%20Object%20Reference) (OtherComp :type Primitive%20Component%20Object%20Reference) (OtherBodyIndex :type Integer) (bFromSweep :type Boolean) (SweepResult :type Hit%20Result%20Structure%20%28by%20ref%29))
  (Utilities|Casting|CastToBP_FirstPersonCharacter OtherActor)
  (Widget|SetVisibility (Variables|/Game/00_Examen_UNIR/WBP_FloorButtonUI.WBP_FloorButtonUI_C|GetText_ButtonMessage (Variables|Default|GetButtonWidget)) "Visible"))

(event OnComponentEndOverlap(Box)
  (params (OverlappedComponent :type Primitive%20Component%20Object%20Reference) (OtherActor :type Actor%20Object%20Reference) (OtherComp :type Primitive%20Component%20Object%20Reference) (OtherBodyIndex :type Integer))
  (Utilities|Casting|CastToBP_FirstPersonCharacter OtherActor)
  (Widget|SetVisibility (Variables|/Game/00_Examen_UNIR/WBP_FloorButtonUI.WBP_FloorButtonUI_C|GetText_ButtonMessage (Variables|Default|GetButtonWidget)) "Hidden"))

(event EventBeginPlay
  (bind _returnvalue (UserInterface|CreateWidget "/Game/00_Examen_UNIR/WBP_FloorButtonUI.WBP_FloorButtonUI_C" (Game|GetPlayerController 0)))
  (bind _output_get (Variables|Default|SetButtonWidget _returnvalue))
  (UserInterface|Viewport|AddtoViewport _output_get 0))

(event Collision|EventActorBeginOverlap
  (params (OtherActor :type Actor%20Object%20Reference)))

(event EventTick
  (params (DeltaSeconds :type Float%20%28single-precision%29)))

(fn ConstructionScript)